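; LevelSpawner builds the ground in BananaCollector by chaining BigGrass level segments end to end.
; On BeginPlay it spawns an initial batch, placing the first segment just below the player pawn and each later one at the newest segment's SpawnPoint.
; Each new segment becomes NewestLevel, receives a reference back to the spawner and randomizes itself through RandomizeLevel.
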(event `self.ReceiveBeginPlay`
  (`self.Spawn Initial Levels`))

(fn `Spawn Initial Levels`
  (bind (_returnvalue_x _returnvalue_y _returnvalue_z) (`KismetMathLibrary.BreakVector` (`self.K2_GetActorLocation` (`GameplayStatics.GetPlayerPawn` 0))))
  (for _ (range 11)
    (`/Engine/EditorBlueprintResources/StandardMacros.IsValid` (`self.Newest Level`)
      (:`Is Valid`
        (`self.SpawnLevelAtSpawnPoint`))
      (:`Is Not Valid`
        (`self.SpawnLevel` (`KismetMathLibrary.MakeVector` _returnvalue_x _returnvalue_y (- _returnvalue_z 100.0)))))))

(fn `SpawnLevel`
  (params (SpawnLocation :type "Vector Structure"))
  (bind _returnvalue (`|SpawnActorFromClass` "/Game/BananaCollector/Blueprints/BigGrass.BigGrass_C" (`KismetMathLibrary.MakeTransform` SpawnLocation) "Undefined" "OverrideRootScale" null null))
  (bind _output_get (set `self.Newest Level` _returnvalue))
  (set `/Game/BananaCollector/Blueprints/BigGrass.LevelSpawner` self _output_get)
  (`/Game/BananaCollector/Blueprints/BigGrass.Randomize Level` _output_get))

(fn `SpawnLevelAtSpawnPoint`
  (`self.SpawnLevel` (`SceneComponent.K2_GetComponentLocation` (`/Game/BananaCollector/Blueprints/BigGrass.SpawnPoint` (`self.Newest Level`)))))

(fn `UserConstructionScript`)