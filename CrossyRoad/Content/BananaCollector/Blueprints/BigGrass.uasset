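; BigGrass is a level segment that randomly becomes grass or road and requests the next segment when the player reaches it.
; RandomizeLevel picks the mesh, then scatters trees on grass or cars on road, tracking them in arrays.
; Player overlap with TriggerZone calls LevelSpawner, destroys the segment, then loops over the trees to destroy them.
; Car cleanup is nested inside the tree loop, so it never runs when TreeArray is empty.
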(event `self.TriggerZone.OnComponentBeginOverlap`
  (params (OverlappedComponent :type "PrimitiveComponent Object Reference") (OtherActor :type "Actor Object Reference") (OtherComp :type "PrimitiveComponent Object Reference") (OtherBodyIndex :type Integer) (bFromSweep :type Boolean) (SweepResult :type "HitResult Structure (by ref)"))
  (cast `/Game/BananaCollector/Blueprints/BP_Player` OtherActor)
  (`/Game/BananaCollector/Blueprints/LevelSpawner.SpawnLevelAtSpawnPoint` (`self.LevelSpawner`))
  (`self.K2_DestroyActor`)
  (for _array_element (`self.Tree Array`)
    (`self.K2_DestroyActor` _array_element)
    (for _array_element_2 (`self.Car Array`)
      (`self.K2_DestroyActor` _array_element_2))))

(fn `Randomize Level`
  (locals (Selection :type Integer))
  (bind (_returnvalue_x _returnvalue_y _returnvalue_z) (`KismetMathLibrary.BreakVector` (`SceneComponent.K2_GetComponentLocation` (`self.StaticMesh`))))
  (bind _returnvalue (+ _returnvalue_y (`KismetMathLibrary.Conv_IntToDouble` (`KismetMathLibrary.RandomIntegerInRange` -3000 3000))))
  (bind _returnvalue_2 (+ _returnvalue_x (`KismetMathLibrary.Conv_IntToDouble` (`KismetMathLibrary.RandomIntegerInRange` 0 100))))
  (bind _returnvalue_3 (+ _returnvalue_z 50.0))
  (bind _output_get (set `local.Selection` (`KismetMathLibrary.RandomIntegerInRange` 0 1)))
  (`StaticMeshComponent.SetStaticMesh` (`self.StaticMesh`) (select `int` _output_get :`0` "/Game/BananaCollector/Meshes/BigGrass.BigGrass" :`1` "/Game/BananaCollector/Meshes/medium_road.medium_road" :!type "StaticMesh Object Reference"))
  (switch `int` _output_get
    (:`0`
      (for _ (range (+ (`KismetMathLibrary.RandomIntegerInRange` 7 40) 1))
        (bind _returnvalue_4 (`|SpawnActorFromClass` "/Game/BananaCollector/Blueprints/Tree.Tree_C" (`KismetMathLibrary.MakeTransform` (`KismetMathLibrary.MakeVector` _returnvalue_2 _returnvalue _returnvalue_3)) "Undefined" "OverrideRootScale" null null))
        (`KismetArrayLibrary.Array_Add` (`self.Tree Array`) _returnvalue_4)))
    (:`1`
      (for _ (range (+ (`KismetMathLibrary.RandomIntegerInRange` 0 3) 1))
        (bind _returnvalue_5 (`|SpawnActorFromClass` "/Game/BananaCollector/Blueprints/Car.Car_C" (`KismetMathLibrary.MakeTransform` (`KismetMathLibrary.MakeVector` _returnvalue_2 _returnvalue _returnvalue_3)) "Undefined" "OverrideRootScale" null null))
        (`KismetArrayLibrary.Array_Add` (`self.Car Array`) _returnvalue_5)))))

(fn `UserConstructionScript`)